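; BP_Tunnel is an endless-runner tunnel segment with a rotating holed wall, plus an enemy and health pack that randomly appear at offset positions.
; Its trigger spawns the next tunnel, destroys this one, raises player speed up to a cap, and scores passes without wall hits.
; Collisions update player health and trigger restart on death, while shot enemies award points.
; RandomizeWall picks one of four hole meshes and a random roll.
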(event `self.ReceiveBeginPlay`
  (bind _enemy (`self.Enemy`))
  (bind _healthpack (`self.HealthPack`))
  (`|ExecutionSequence`
    (:`then_0`
      (`|ExecutionSequence`
        (:`then_0`
          (if (!= (`KismetMathLibrary.RandomIntegerInRange` 0 1) 0)
            (`PrimitiveComponent.SetCollisionEnabled` _enemy "NoCollision")
            (`SceneComponent.SetVisibility` _enemy false false)))
        (:`then_1`
          (`SceneComponent.K2_AddWorldOffset` _enemy (`KismetMathLibrary.MakeVector` (`KismetMathLibrary.RandomFloatInRange` -250.0 250.0) (`KismetMathLibrary.RandomFloatInRange` -250.0 250.0) (`KismetMathLibrary.RandomFloatInRange` -250.0 250.0)) false false))
        (:`then_2`
          (`KismetSystemLibrary.Delay` 15.0)
          (`ActorComponent.K2_DestroyComponent` (`self.Enemy`)))))
    (:`then_1`
      (`|ExecutionSequence`
        (:`then_0`
          (if (!= (`KismetMathLibrary.RandomIntegerInRange` 0 1) 0)
            (`PrimitiveComponent.SetCollisionEnabled` _healthpack "NoCollision")
            (`SceneComponent.SetVisibility` _healthpack false false)))
        (:`then_1`
          (`SceneComponent.K2_AddWorldOffset` (`self.HealthPack`) (`KismetMathLibrary.MakeVector` (`KismetMathLibrary.RandomFloatInRange` -250.0 250.0) (`KismetMathLibrary.RandomFloatInRange` -250.0 250.0) (`KismetMathLibrary.RandomFloatInRange` -250.0 250.0)) false false))
        (:`then_2`
          (`KismetSystemLibrary.Delay` 15.0)
          (`ActorComponent.K2_DestroyComponent` (`self.HealthPack`)))))))

(event `self.ReceiveTick`
  (params (DeltaSeconds :type "Float (single-precision)"))
  (`SceneComponent.K2_AddLocalRotation` (`self.WallMesh`) (`KismetMathLibrary.MakeRotator` (* DeltaSeconds (`self.RotateSpeed`))) false false))

(event `self.TriggerZone.OnComponentBeginOverlap`
  (params (OverlappedComponent :type "PrimitiveComponent Object Reference") (OtherActor :type "Actor Object Reference") (OtherComp :type "PrimitiveComponent Object Reference") (OtherBodyIndex :type Integer) (bFromSweep :type Boolean) (SweepResult :type "HitResult Structure (by ref)"))
  (bind _asbp_player (cast `/Game/InfiniteMatrix/Blueprints/BP_Player` OtherActor))
  (`|ExecutionSequence`
    (:`then_0`
      (`/Game/InfiniteMatrix/Blueprints/BP_TunnelSpawner.SpawnTunnelAtSpawnPoint` (`self.TunnelSpawner`))
      (`self.K2_DestroyActor`))
    (:`then_1`
      (set `/Game/InfiniteMatrix/Blueprints/BP_Player.ForwardSpeed` (`KismetMathLibrary.FMin` (+ (`/Game/InfiniteMatrix/Blueprints/BP_Player.ForwardSpeed` _asbp_player) 40.0) 4000.0) _asbp_player))))

(event `self.WallMesh.OnComponentBeginOverlap`
  (params (OverlappedComponent :type "PrimitiveComponent Object Reference") (OtherActor :type "Actor Object Reference") (OtherComp :type "PrimitiveComponent Object Reference") (OtherBodyIndex :type Integer) (bFromSweep :type Boolean) (SweepResult :type "HitResult Structure (by ref)"))
  (bind _asbp_player (cast `/Game/InfiniteMatrix/Blueprints/BP_Player` (stale `self.WallMesh.OnComponentHit` OtherActor) :!label _label))
  (if (and (not (`/Game/InfiniteMatrix/Blueprints/BP_Player.IsDead` _asbp_player)) (not (`self.UserHasHitWall`)))
    (set `self.UserHasHitWall` true)
    (bind _output_get (set `/Game/InfiniteMatrix/Blueprints/BP_Player.Health` (- (`/Game/InfiniteMatrix/Blueprints/BP_Player.Health` _asbp_player) 25) _asbp_player))
    (`/Game/InfiniteMatrix/UI/WB_Healthbar.UpdateHealthbar` (`/Game/InfiniteMatrix/Blueprints/BP_Player.WB_Healthbar` _asbp_player) _output_get)
    (if (<= _output_get 0)
      (set `/Game/InfiniteMatrix/Blueprints/BP_Player.IsDead` true _asbp_player)
      (`/Game/InfiniteMatrix/Blueprints/BP_Player.DisplayRestart` _asbp_player))))

(event `self.WallMesh.OnComponentHit`
  (params (HitComponent :type "PrimitiveComponent Object Reference") (OtherActor :type "Actor Object Reference") (OtherComp :type "PrimitiveComponent Object Reference") (NormalImpulse :type "Vector Structure") (Hit :type "HitResult Structure (by ref)"))
  (`|ExecutionSequence`
    (:`then_0`
      (goto _label))
    (:`then_1`
      (`KismetSystemLibrary.Delay` 0.3)
      (`PrimitiveComponent.SetCollisionEnabled` (`self.WallMesh`) "NoCollision"))))

(event `self.TriggerZone.OnComponentEndOverlap`
  (params (OverlappedComponent :type "PrimitiveComponent Object Reference") (OtherActor :type "Actor Object Reference") (OtherComp :type "PrimitiveComponent Object Reference") (OtherBodyIndex :type Integer))
  (bind _asbp_player (cast `/Game/InfiniteMatrix/Blueprints/BP_Player` OtherActor))
  (if (not (`self.UserHasHitWall`))
    (bind _result (`/Engine/EditorBlueprintResources/StandardMacros.IncrementInt` (`/Game/InfiniteMatrix/Blueprints/BP_Player.Score` _asbp_player))
      (:`  `
        (set `/Game/InfiniteMatrix/Blueprints/BP_Player.Score` _result _asbp_player)))))

(event `self.HealthPack.OnComponentBeginOverlap`
  (params (OverlappedComponent :type "PrimitiveComponent Object Reference") (OtherActor :type "Actor Object Reference") (OtherComp :type "PrimitiveComponent Object Reference") (OtherBodyIndex :type Integer) (bFromSweep :type Boolean) (SweepResult :type "HitResult Structure (by ref)"))
  (bind _asbp_player (cast `/Game/InfiniteMatrix/Blueprints/BP_Player` OtherActor))
  (`|ExecutionSequence`
    (:`then_0`
      (bind _returnvalue (+ (`/Game/InfiniteMatrix/Blueprints/BP_Player.Health` _asbp_player) 25))
      (if (>= _returnvalue 100)
        (set `/Game/InfiniteMatrix/Blueprints/BP_Player.Health` 100 _asbp_player)
        (else
          (bind _output_get (set `/Game/InfiniteMatrix/Blueprints/BP_Player.Health` _returnvalue _asbp_player))))
      (`/Game/InfiniteMatrix/UI/WB_Healthbar.UpdateHealthbar` (`/Game/InfiniteMatrix/Blueprints/BP_Player.WB_Healthbar` _asbp_player) _output_get))
    (:`then_1`
      (`ActorComponent.K2_DestroyComponent` (`self.HealthPack`)))))

(event `self.Enemy.OnComponentHit`
  (params (HitComponent :type "PrimitiveComponent Object Reference") (OtherActor :type "Actor Object Reference") (OtherComp :type "PrimitiveComponent Object Reference") (NormalImpulse :type "Vector Structure") (Hit :type "HitResult Structure (by ref)"))
  (bind _asbp_player (cast `/Game/InfiniteMatrix/Blueprints/BP_Player` OtherActor :!label _label_2)
    (:`then`
      (`|ExecutionSequence`
        (:`then_0`
          (bind _result (`/Engine/EditorBlueprintResources/StandardMacros.IncrementInt` (`/Game/InfiniteMatrix/Blueprints/BP_Player.EnemiesHit` _asbp_player))
            (:`  `
              (set `/Game/InfiniteMatrix/Blueprints/BP_Player.EnemiesHit` _result _asbp_player))))
        (:`then_1`
          (`ActorComponent.K2_DestroyComponent` (`self.Enemy`))
          (if (and (not (`/Game/InfiniteMatrix/Blueprints/BP_Player.IsDead` _asbp_player)) (not (`self.UserHasHitWall`)))
            (set `self.UserHasHitEnemy` true)
            (bind _output_get (set `/Game/InfiniteMatrix/Blueprints/BP_Player.Health` (- (`/Game/InfiniteMatrix/Blueprints/BP_Player.Health` _asbp_player) 15) _asbp_player))
            (`/Game/InfiniteMatrix/UI/WB_Healthbar.UpdateHealthbar` (`/Game/InfiniteMatrix/Blueprints/BP_Player.WB_Healthbar` _asbp_player) _output_get)
            (if (<= _output_get 0)
              (set `/Game/InfiniteMatrix/Blueprints/BP_Player.IsDead` true _asbp_player)
              (`/Game/InfiniteMatrix/Blueprints/BP_Player.DisplayRestart` _asbp_player))))))
    (:`CastFailed`
      (`|ExecutionSequence`
        (:`then_0`
          (bind _asbp_player_2 (cast `/Game/InfiniteMatrix/Blueprints/BP_Player` (`GameplayStatics.GetPlayerPawn` 0)))
          (bind _result_2 (`/Engine/EditorBlueprintResources/StandardMacros.IncrementInt` (`/Game/InfiniteMatrix/Blueprints/BP_Player.Score` _asbp_player_2))
            (:`  `
              (set `/Game/InfiniteMatrix/Blueprints/BP_Player.Score` _result_2 _asbp_player_2)
              (`ActorComponent.K2_DestroyComponent` (`self.Enemy`)))))
        (:`then_1`
          (bind _asbp_projectile (cast `/Game/InfiniteMatrix/Blueprints/BP_Projectile` (stale `self.Enemy.OnComponentBeginOverlap` OtherActor)))
          (`ActorComponent.K2_DestroyComponent` (`/Game/InfiniteMatrix/Blueprints/BP_Projectile.Sphere` _asbp_projectile)))
        (:`then_2`
          (bind _result_3 (`/Engine/EditorBlueprintResources/StandardMacros.IncrementInt` (`/Game/InfiniteMatrix/Blueprints/BP_Player.EnemiesDestroyed` _asbp_player_2))
            (:`  `
              (set `/Game/InfiniteMatrix/Blueprints/BP_Player.EnemiesDestroyed` _result_3 _asbp_player_2))))))))

(event `self.Enemy.OnComponentBeginOverlap`
  (params (OverlappedComponent :type "PrimitiveComponent Object Reference") (OtherActor :type "Actor Object Reference") (OtherComp :type "PrimitiveComponent Object Reference") (OtherBodyIndex :type Integer) (bFromSweep :type Boolean) (SweepResult :type "HitResult Structure (by ref)"))
  (goto _label_2))

(fn `RandomizeWall`
  (`StaticMeshComponent.SetStaticMesh` (`self.WallMesh`) (select `int` (`KismetMathLibrary.RandomIntegerInRange` 0 3) :`0` "/Game/InfiniteMatrix/Meshes/SM_Hole_01.SM_Hole_01" :`1` "/Game/InfiniteMatrix/Meshes/SM_Hole_02.SM_Hole_02" :`2` "/Game/InfiniteMatrix/Meshes/SM_Hole_03.SM_Hole_03" :`3` "/Game/InfiniteMatrix/Meshes/SM_Hole_04.SM_Hole_04" :!type "StaticMesh Object Reference"))
  (`SceneComponent.K2_AddLocalRotation` (`self.WallMesh`) (`KismetMathLibrary.MakeRotator` (`KismetMathLibrary.RandomFloatInRange` 0.0 360.0)) false false))

(fn `UserConstructionScript`)